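; BP_TP_Character is a player character, apparently third-person by its name, that handles basic move, look and crouch input.
; Movement axes follow control yaw only, calling forced AddMovementInput scaled by MovementSpeed and delta time.
; Look axes feed controller pitch and yaw scaled by LookSpeed and delta time.
; A FlipFlop on the Crouch press toggles between crouching and standing.
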(event `InputAxis|MoveForward`
  (params (AxisValue :type "Float (single-precision)"))
  ;[0.1014 0.326 1] Move
  (`self.AddMovementInput` (`KismetMathLibrary.GetForwardVector` (`KismetMathLibrary.MakeRotator` 0.0 0.0 (.yaw (`self.GetControlRotation`)))) (* (* (`self.MovementSpeed`) (`GameplayStatics.GetWorldDeltaSeconds`)) AxisValue) true))

(event `InputAxis|MoveRight`
  (params (AxisValue :type "Float (single-precision)"))
  ;[0.1014 0.326 1] Move
  (`self.AddMovementInput` (`KismetMathLibrary.GetRightVector` (`KismetMathLibrary.MakeRotator` 0.0 0.0 (.yaw (`self.GetControlRotation`)))) (* (* (`self.MovementSpeed`) (`GameplayStatics.GetWorldDeltaSeconds`)) AxisValue) true))

(event `InputAction|Crouch`
  (params (Key :type "Key Structure"))
  ;[0.1014 0.326 1] Crouch
  (:`Pressed`
    (`/Engine/EditorBlueprintResources/StandardMacros.FlipFlop`
      (:`A`
        (`self.Crouch`))
      (:`B`
        (`self.UnCrouch`)))))

(event `InputAxis|LookPitch`
  (params (AxisValue :type "Float (single-precision)"))
  ;[0.1014 0.326 1] Look
  (`self.AddControllerPitchInput` (* (* (`self.LookSpeed`) (`GameplayStatics.GetWorldDeltaSeconds`)) AxisValue)))

(event `InputAxis|LookYaw`
  (params (AxisValue :type "Float (single-precision)"))
  ;[0.1014 0.326 1] Look
  (`self.AddControllerYawInput` (* (* (`self.LookSpeed`) (`GameplayStatics.GetWorldDeltaSeconds`)) AxisValue)))

(fn `UserConstructionScript`)